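; Actor component that constrains its owning Character to move along a spline, such as for path-locked movement.
; StartTravelingSpline and StopTravelingSpline set or clear the active spline and a traveling flag.
; AddMovementInputAlongSpline feeds movement input along the spline direction nearest the character.
; It then snaps the character's X and Y onto that nearest spline point, preserving Z so height stays free.
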(event EventBeginPlay
  (bind _ascharacter (Utilities|Casting|CastToCharacter (Components|GetOwner)))
  (Variables|Default|SetCharacter _ascharacter))

(fn StartTravelingSpline
  (params (SplineComponent :type Spline%20Component%20Object%20Reference))
  (if (Variables|Default|GetIsTravelingSpline)
    (CallFunction|StopTravelingSpline))
  (Variables|Default|SetSplineInUse SplineComponent)
  (Variables|Default|SetIsTravelingSpline true))

(fn StopTravelingSpline
  (Variables|Default|SetIsTravelingSpline false)
  (Variables|Default|SetSplineInUse 0))

(fn AddMovementInputAlongSpline
  (params (ScaleValue :type Float%20%28single-precision%29))
  (bind _splineinuse (Variables|Default|GetSplineInUse)
    (:then
      (Pawn|Input|AddMovementInput (Variables|Default|GetCharacter) (Spline|GetDirectionatDistanceAlongSpline _splineinuse (Class|SplineComponent|GetDistanceAlongSplineatLocation _splineinuse (Transformation|GetActorLocation (Variables|Default|GetCharacter)) "World") "World") ScaleValue false)
      (Transformation|SetActorLocation (Variables|Default|GetCharacter) (Math|Vector|MakeVector (.x (Spline|GetLocationatDistanceAlongSpline _splineinuse (Class|SplineComponent|GetDistanceAlongSplineatLocation _splineinuse (Transformation|GetActorLocation (Variables|Default|GetCharacter)) "World") "World")) (.y (Spline|GetLocationatDistanceAlongSpline _splineinuse (Class|SplineComponent|GetDistanceAlongSplineatLocation _splineinuse (Transformation|GetActorLocation (Variables|Default|GetCharacter)) "World") "World")) (.z (Transformation|GetActorLocation (Variables|Default|GetCharacter)))) false false))
    (:else)))