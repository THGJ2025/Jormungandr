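; Actor component that gives its owner a health pool with damage, healing and death.
; On BeginPlay it binds to the owner's OnTakeAnyDamage and applies incoming damage unless the owner is already dead.
; Heal, Kill and TakeDamage all route through SetHealth, which broadcasts health changes and fires OnDeath at zero.
; Heal clamps to MaxHealth, and separate dispatchers report damage and healing amounts.
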(event Custom|OnTakeAnyDamage_Event
  (params (DamagedActor :type Actor%20Object%20Reference) (Damage :type Float%20%28single-precision%29) (DamageType :type Damage%20Type%20Object%20Reference) (InstigatedBy :type Controller%20Object%20Reference) (DamageCauser :type Actor%20Object%20Reference))
  (if (not (CallFunction|IsDead))
    (CallFunction|TakeDamage Damage DamageCauser)))

(event EventBeginPlay
  (EventDispatchers|AssignOnTakeAnyDamage (Components|GetOwner) (delegate Custom|OnTakeAnyDamage_Event)))

(fn Heal
  (params (Amount :type Float%20%28double-precision%29))
  (CallFunction|SetHealth (Math|Float|Clamp(Float) (+ (Variables|Default|GetHealth) Amount) 0.0 (Variables|Default|GetMaxHealth)))
  (Default|CallOnHealed Amount))

(fn Kill
  (CallFunction|SetHealth 0.0))

(fn SetHealth
  (params (NewHealth :type Float%20%28double-precision%29))
  (bind _output_get (Variables|Default|SetHealth NewHealth))
  (Default|CallOnHealthChanged _output_get)
  (if (<= _output_get 0.0)
    (Default|CallOnDeath)))

(fn TakeDamage
  (params (Damage :type Float%20%28double-precision%29) (DamageCauser :type Actor%20Object%20Reference))
  (CallFunction|SetHealth (Math|Float|Max(Float) (- (Variables|Default|GetHealth) Damage) 0.0))
  (Default|CallOnDamaged Damage DamageCauser))

(fn IsDead
  (return (<= (Variables|Default|GetHealth) 0.0)))