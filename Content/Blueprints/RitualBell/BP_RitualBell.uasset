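; BP_RitualBell is a ritual bell actor that can be detached from its parent and launched as a spinning projectile.
; LaunchBell sets the projectile velocity, detaches the actor, places it at the given position and rotation, activates projectile and rotating movement, and flags it as launched.
; A box collision hit event only prints the hit actor's name and is commented as not working.
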(event OnComponentHit(BoxCollision)
  (params (HitComponent :type Primitive%20Component%20Object%20Reference) (OtherActor :type Actor%20Object%20Reference) (OtherComp :type Primitive%20Component%20Object%20Reference) (NormalImpulse :type Vector :default "0, 0, 0") (Hit :type Hit%20Result%20Structure%20%28by%20ref%29))
  ;[0.15 0 0.1036 0.5] doesnt work
  (Development|PrintString (Utilities|GetDisplayName (.hitactor Hit))))

(fn ConstructionScript)

(fn LaunchBell
  (params (Velocity :type Vector) (Posiiton :type Vector) (Rotation :type Rotator))
  (Variables|/Script/Engine.MovementComponent|SetVelocity (Variables|Default|GetProjectileMovement) Velocity)
  (Transformation|DetachFromActor "KeepWorld" "KeepRelative" "KeepRelative")
  (Transformation|SetActorLocation Posiiton false false)
  (Transformation|SetActorRotation Rotation)
  (Components|Activation|Activate (Variables|Default|GetProjectileMovement) false)
  (Variables|Default|SetbLaunched true)
  (Components|Activation|Activate (Variables|Default|GetRotatingMovement) false))