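; Two-way tunnel path actor that pairs a placed BP_TunnelSpline with a runtime-generated reversed copy, so each direction has its own interactable spline.
; The construction script caches and updates the child actor spline.
; BeginPlay spawns a second child actor at the last point and rebuilds it from the reversed world-space point positions.
; Start and stop events from either spline toggle IsInUse and interaction on both, locking the path during use.
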(event Custom|OnStartUsing_Event
  (Variables|Default|SetIsInUse true)
  (Class|JInteractInterface|SetCanInteract (Variables|Default|GetBaseSpline) false))

(event Custom|OnStopUsing_Event
  (Class|JInteractInterface|SetCanInteract (Variables|Default|GetReversedSpline) true)
  (Variables|Default|SetIsInUse false))

(event EventBeginPlay
  (Utilities|FlowControl|Sequence
    (:then_0
      (CallFunction|CloneBaseSpline))
    (:then_1
      (EventDispatchers|AssignOnStartUsing (Variables|Default|GetBaseSpline) (delegate Custom|OnStartUsing_Event))
      (EventDispatchers|AssignOnStopUsing (Variables|Default|GetBaseSpline) (delegate Custom|OnStopUsing_Event)))))

(fn ConstructionScript
  (bind _asbp_tunnel_spline (Utilities|Casting|CastToBP_TunnelSpline (Variables|/Script/Engine.ChildActorComponent|GetChildActor (Variables|Default|GetTunnelSpline))))
  (bind _output_get (Variables|Default|SetBaseSpline _asbp_tunnel_spline))
  (Default|Update _output_get))

(fn CloneBaseSpline
  (bind _basespline (Variables|Default|GetBaseSpline))
  (bind _splinecomponent (Variables|/Game/Blueprints/Environment/BP_TunnelSpline.BP_TunnelSpline_C|GetSplineComponent _basespline))
  (bind _returnvalue (AddComponent|AddChildActorComponent false))
  (Transformation|SetWorldLocation _returnvalue (Spline|GetLocationatSplinePoint _splinecomponent (- (Spline|GetNumberOfSplinePoints _splinecomponent) 1) "World") false false)
  (bind _asbp_tunnel_spline (Utilities|Casting|CastToBP_TunnelSpline (Variables|/Script/Engine.ChildActorComponent|GetChildActor _returnvalue)))
  (bind _output_get (Variables|Default|SetReversedSpline _asbp_tunnel_spline))
  (Spline|ClearSplinePoints (Variables|/Game/Blueprints/Environment/BP_TunnelSpline.BP_TunnelSpline_C|GetSplineComponent _output_get) false)
  (bind _output_get_2 (LocalVariables|SetSplinePointsPosition (CallFunction|GetSplinePointsLocation "World")))
  (Utilities|Array|Reverse _output_get_2)
  (Spline|SetSplinePoints (Variables|/Game/Blueprints/Environment/BP_TunnelSpline.BP_TunnelSpline_C|GetSplineComponent (Variables|Default|GetReversedSpline)) (LocalVariables|GetSplinePointsPosition) "World" true)
  (Default|Update (Variables|Default|GetReversedSpline)))

(fn GetSplinePointsLocation
  (params (CoordinateSpace :type ESplineCoordinateSpace%20Enum :default "Local"))
  (bind _basespline (Variables|Default|GetBaseSpline))
  (bind _splinecomponent (Variables|/Game/Blueprints/Environment/BP_TunnelSpline.BP_TunnelSpline_C|GetSplineComponent _basespline))
  (for _index (range 0 (- (Spline|GetNumberOfSplinePoints _splinecomponent) 1))
    (Utilities|Array|Add (LocalVariables|GetSplinePoints) (Spline|GetLocationatSplinePoint _splinecomponent _index CoordinateSpace)))
  (return (LocalVariables|GetSplinePoints)))