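; Banishing circle interactable that the player completes by placing a missing crystal, enabling a draugr-soothing ritual that so far only prints debug messages.
; Interacting spawns a temporary crystal mesh at the player, lerps it into place via timeline, then reveals the real one.
; Overlapping RitualArea then starts a looping timer counting saved entities against a draugr count randomly re-rolled each tick.
; Ending overlap resets an unfinished ritual; reaching the count finishes it permanently.
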(event OnComponentBeginOverlap(RitualArea)
  (params (OverlappedComponent :type Primitive%20Component%20Object%20Reference) (OtherActor :type Actor%20Object%20Reference) (OtherComp :type Primitive%20Component%20Object%20Reference) (OtherBodyIndex :type Integer) (bFromSweep :type Boolean) (SweepResult :type Hit%20Result%20Structure%20%28by%20ref%29))
  (if (Variables|Default|GetIsCompleted)
    (if (not (Variables|Default|GetIsRitualDone))
      (Variables|Default|SetIsInRitual true)
      (bind _returnvalue (Utilities|Time|SetTimerbyEvent (delegate Custom|RitualLoop) (Variables|Default|GetSoothingDuration) true))
      (Variables|Default|SetRitualTimer _returnvalue))))

(event OnComponentEndOverlap(RitualArea)
  (params (OverlappedComponent :type Primitive%20Component%20Object%20Reference) (OtherActor :type Actor%20Object%20Reference) (OtherComp :type Primitive%20Component%20Object%20Reference) (OtherBodyIndex :type Integer))
  (if (Variables|Default|GetIsInRitual)
    (CallFunction|EndRitual)))

(event Custom|RitualLoop
  (Development|PrintString "Saving daugrh")
  (bind _result (Math|Integer|IncrementInt (Variables|Default|GetEntitiesSaved))
    (:%20%20
      (if (>= _result (CallFunction|GetDraugrCount))
        (Variables|Default|SetIsRitualDone true)
        (CallFunction|EndRitual)
        (Development|PrintString "Ritual ended")))))

(event EventBeginPlay)

(event Collision|EventActorBeginOverlap
  (params (OtherActor :type Actor%20Object%20Reference)))

(event EventTick
  (params (DeltaSeconds :type Float%20%28single-precision%29)))

(event EventInteractPressCompleted
  (bind _returnvalue (Game|GetPlayerCharacter 0))
  (if (not (Variables|Default|GetIsCompleted))
    (bind _asbp_player (Utilities|Casting|CastToBP_Player (Game|GetPlayerCharacter 0)))
    (Variables|Default|SetIsCompleted true)
    (Class|JInteractInterface|SetCanInteract false)
    (bind _output_get (Variables|Default|SetStartTransform (Math|Transform|MakeTransform (Transformation|GetActorLocation _returnvalue) (Transformation|GetActorRotation _returnvalue) (Transformation|GetWorldScale (Variables|Default|GetMissingCrystal)))))
    (bind _returnvalue_2 (Game|SpawnActorfromClass "/Script/Engine.StaticMeshActor" _output_get "AlwaysSpawn" "MultiplyWithRoot" 0 0))
    (bind _output_get_2 (Variables|Default|SetTempMesh _returnvalue_2))
    (Transformation|SetMobility _output_get_2 "Movable")
    (Components|StaticMesh|SetStaticMesh (Variables|/Script/Engine.StaticMeshActor|GetStaticMeshComponent _output_get_2) "/Game/Assets/StaticMesh/Crystal_Low_02.Crystal_Low_02")
    (Collision|SetActorEnableCollision _output_get_2 false)
    (bind _alpha (Timeline|Timeline Play)
      (:Update
        (Transformation|SetActorTransform (Variables|Default|GetTempMesh) (Math|Transform|Lerp(Transform) (Variables|Default|GetStartTransform) (Transformation|GetWorldTransform (Variables|Default|GetMissingCrystal)) _alpha)))
      (:Finished
        (Collision|SetCollisionProfileName (Variables|Default|GetMissingCrystal) "BlockAllDynamic" true :!class /Script/Engine.PrimitiveComponent)
        (Rendering|SetVisibility (Variables|Default|GetMissingCrystal) true false)
        (Actor|DestroyActor (Variables|Default|GetTempMesh))))))

(fn ConstructionScript)

(fn GetDraugrCount
  (return (Math|Random|RandomIntegerinRange 2 5)))

(fn GetWidgetAttachmentComponent
  (return (Variables|Default|GetInteractArea)))

(fn EndRitual
  (Variables|Default|SetIsInRitual false)
  (Utilities|Time|ClearandInvalidateTimerbyHandle (Variables|Default|GetRitualTimer))
  (Variables|Default|SetEntitiesSaved 0)
  (Development|PrintString "Reset ritual"))