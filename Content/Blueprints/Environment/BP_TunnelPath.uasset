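; BP_TunnelPath is a spline-based tunnel that the player can travel through from either end.
; The construction script places and orients an overlap volume at the first and last spline points, and BeginPlay builds a reversed copy of the spline from its point locations.
; Overlapping either volume stops a player already traveling a spline, or otherwise starts travel on the base or reversed spline, matching the entry end.
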(event OnComponentBeginOverlap(BVolume)
  (params (OverlappedComponent :type Primitive%20Component%20Object%20Reference) (OtherActor :type Actor%20Object%20Reference) (OtherComp :type Primitive%20Component%20Object%20Reference) (OtherBodyIndex :type Integer) (bFromSweep :type Boolean) (SweepResult :type Hit%20Result%20Structure%20%28by%20ref%29))
  (bind _asbp_player (Utilities|Casting|CastToBP_Player OtherActor))
  (if (Variables|/Game/Blueprints/Components/AC_CharacterSplineMovement.AC_CharacterSplineMovement_C|GetIsTravelingSpline (Variables|/Game/Blueprints/Player/BP_Player.BP_Player_C|GetCharacterSplineMovement _asbp_player))
    (Default|StopTravelingTunnel _asbp_player)
    (else
      (Default|StartTravelingTunnel _asbp_player (Variables|Default|GetReversedSpline)))))

(event OnComponentBeginOverlap(AVolume)
  (params (OverlappedComponent :type Primitive%20Component%20Object%20Reference) (OtherActor :type Actor%20Object%20Reference) (OtherComp :type Primitive%20Component%20Object%20Reference) (OtherBodyIndex :type Integer) (bFromSweep :type Boolean) (SweepResult :type Hit%20Result%20Structure%20%28by%20ref%29))
  (bind _asbp_player (Utilities|Casting|CastToBP_Player OtherActor))
  (if (Variables|/Game/Blueprints/Components/AC_CharacterSplineMovement.AC_CharacterSplineMovement_C|GetIsTravelingSpline (Variables|/Game/Blueprints/Player/BP_Player.BP_Player_C|GetCharacterSplineMovement _asbp_player))
    (Default|StopTravelingTunnel _asbp_player)
    (else
      (Default|StartTravelingTunnel _asbp_player (Variables|Default|GetBaseSpline)))))

(event EventBeginPlay
  (CallFunction|CloneBaseSpline))

(fn ConstructionScript
  (bind _basespline (Variables|Default|GetBaseSpline))
  (bind _basespline_2 (Variables|Default|GetBaseSpline))
  (bind _returnvalue (Spline|GetNumberOfSplinePoints _basespline))
  (bind _returnvalue_2 (- _returnvalue 1))
  ;[0.15 0.15 0.15 0.5] Init 2 volume pos for end of path
  (Transformation|SetRelativeTransform (Variables|Default|GetAVolume) (Math|Transform|MakeTransform (Spline|GetLocationatSplinePoint _basespline_2 0 "Local") (Math|Rotator|MakeRotfromX (Class|SplineComponent|GetDirectionatSplinePoint _basespline_2 0 "Local")) "1.000000,1.000000,1.000000") false false)
  (Transformation|SetRelativeTransform (Variables|Default|GetBVolume) (Math|Transform|MakeTransform (Spline|GetLocationatSplinePoint _basespline _returnvalue_2 "Local") (Math|Rotator|MakeRotfromX (Class|SplineComponent|GetDirectionatSplinePoint _basespline _returnvalue_2 "Local")) "1.000000,1.000000,1.000000") false false))

(fn CloneBaseSpline
  (bind _returnvalue (AddComponent|AddSplineComponent false))
  (bind _output_get (Variables|Default|SetReversedSpline _returnvalue))
  (Spline|ClearSplinePoints _output_get false)
  (bind _output_get_2 (LocalVariables|SetSplinePointsPosition (CallFunction|GetSplinePointsLocation "World")))
  (Utilities|Array|Reverse _output_get_2)
  (Spline|SetSplinePoints (Variables|Default|GetReversedSpline) (LocalVariables|GetSplinePointsPosition) "World" true))

(fn GetSplinePointsLocation
  (params (CoordinateSpace :type ESplineCoordinateSpace%20Enum :default "Local"))
  (for _index (range 0 (- (Spline|GetNumberOfSplinePoints (Variables|Default|GetBaseSpline)) 1))
    (Utilities|Array|Add (LocalVariables|GetSplinePoints) (Spline|GetLocationatSplinePoint (Variables|Default|GetBaseSpline) _index CoordinateSpace)))
  (return (LocalVariables|GetSplinePoints)))