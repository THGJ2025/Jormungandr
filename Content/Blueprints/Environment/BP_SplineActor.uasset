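; BP_SplineActor is an environment actor that wraps a Spline component behind a small function API for other objects to query and edit.
; Pass-through functions clear or insert points and return point count, point data, locations, direction at a distance and distance at a location.
; GetStartLocation and GetEndLocation add shortcuts to the first and last spline points.
; The event graph and construction script are empty.
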(event EventBeginPlay)

(event Collision|EventActorBeginOverlap
  (params (OtherActor :type Actor%20Object%20Reference)))

(event EventTick
  (params (DeltaSeconds :type Float%20%28single-precision%29)))

(fn ConstructionScript)

(fn ClearSplinePoints
  (params (bUpdateSpline :type Boolean))
  (Spline|ClearSplinePoints (Variables|Default|GetSpline) bUpdateSpline))

(fn GetNumberOfSplinePoints
  (return (Spline|GetNumberOfSplinePoints (Variables|Default|GetSpline))))

(fn GetSplinePointat
  (params (PointIndex :type Integer) (CoordinateSpace :type ESplineCoordinateSpace%20Enum :default "Local"))
  (return (Spline|GetSplinePointAt (Variables|Default|GetSpline) PointIndex CoordinateSpace)))

(fn AddSplinePointatIndex
  (params (Position :type Vector%20%28by%20ref%29) (Index :type Integer) (CoordinateSpace :type ESplineCoordinateSpace%20Enum :default "Local") (bUpdateSpline :type Boolean))
  (Spline|AddSplinePointatIndex (Variables|Default|GetSpline) Position Index CoordinateSpace bUpdateSpline))

(fn GetLocationatSplinePoint
  (params (PointIndex :type Integer) (CoordinateSpace :type ESplineCoordinateSpace%20Enum :default "Local"))
  (return (Spline|GetLocationatSplinePoint (Variables|Default|GetSpline) PointIndex CoordinateSpace)))

(fn GetDirectionatDistanceAlongSpline
  (params (Distance :type Float%20%28single-precision%29) (CoordinateSpace :type ESplineCoordinateSpace%20Enum :default "Local"))
  (return (Spline|GetDirectionatDistanceAlongSpline (Variables|Default|GetSpline) Distance CoordinateSpace)))

(fn GetStartLocation
  (params (CoordinateSpace :type ESplineCoordinateSpace%20Enum :default "Local"))
  (return (Spline|GetLocationatSplinePoint (Variables|Default|GetSpline) 0 CoordinateSpace)))

(fn GetEndLocation
  (params (CoordinateSpace :type ESplineCoordinateSpace%20Enum :default "Local"))
  (return (Spline|GetLocationatSplinePoint (Variables|Default|GetSpline) (- (CallFunction|GetNumberOfSplinePoints) 1) CoordinateSpace)))

(fn GetDistanceAlongSplineatLocation
  (params (InLocation :type Vector%20%28by%20ref%29) (CoordinateSpace :type ESplineCoordinateSpace%20Enum :default "Local"))
  (return (Class|SplineComponent|GetDistanceAlongSplineatLocation (Variables|Default|GetSpline) InLocation CoordinateSpace)))