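; Interactable tunnel path that sends the player traveling along its spline and releases them on reaching either end.
; The construction script snaps the start and end trigger volumes to the first and last spline points, aligned with the spline direction.
; Interacting disables interaction, starts BP_Player tunnel travel and registers the player.
; Overlapping an end volume unregisters any tracked actor with a notification, stopping travel and re-enabling interaction for the player.
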(event OnComponentBeginOverlap(StartVolume)
  (params (OverlappedComponent :type Primitive%20Component%20Object%20Reference) (OtherActor :type Actor%20Object%20Reference) (OtherComp :type Primitive%20Component%20Object%20Reference) (OtherBodyIndex :type Integer) (bFromSweep :type Boolean) (SweepResult :type Hit%20Result%20Structure%20%28by%20ref%29))
  (if (CallFunction|IsActoronSpline OtherActor)
    (CallFunction|LeaveSpline OtherActor)
    ;[0.15 0.15 0.15 0.5] Player leave spline
    (if (== (Game|GetPlayerCharacter 0) OtherActor)
      (bind _asbp_player (Utilities|Casting|CastToBP_Player OtherActor))
      (Default|StopTravelingTunnel _asbp_player)
      (Class|JInteractInterface|SetCanInteract true))))

(event OnComponentBeginOverlap(EndVolume)
  (params (OverlappedComponent :type Primitive%20Component%20Object%20Reference) (OtherActor :type Actor%20Object%20Reference) (OtherComp :type Primitive%20Component%20Object%20Reference) (OtherBodyIndex :type Integer) (bFromSweep :type Boolean) (SweepResult :type Hit%20Result%20Structure%20%28by%20ref%29))
  (if (CallFunction|IsActoronSpline OtherActor)
    (CallFunction|LeaveSpline OtherActor)
    ;[0.15 0.15 0.15 0.5] Player leave spline
    (if (== (Game|GetPlayerCharacter 0) OtherActor)
      (bind _asbp_player (Utilities|Casting|CastToBP_Player OtherActor))
      (Default|StopTravelingTunnel _asbp_player)
      (Class|JInteractInterface|SetCanInteract true))))

(event EventBeginPlay)

(event EventInteractPressCompleted
  (bind _returnvalue (Game|GetPlayerCharacter 0))
  (if (not (CallFunction|IsActoronSpline _returnvalue))
    (bind _asbp_player (Utilities|Casting|CastToBP_Player _returnvalue))
    (if true
      (Class|JInteractInterface|SetCanInteract false)
      (Default|StartTravelingTunnel _asbp_player (Variables|Default|GetSplineComponent))
      (CallFunction|JoinSpline _asbp_player))))

(fn ConstructionScript
  (CallFunction|Update))

(fn Update
  (bind _splinecomponent (Variables|Default|GetSplineComponent))
  (bind _splinecomponent_2 (Variables|Default|GetSplineComponent))
  (bind _returnvalue (Spline|GetNumberOfSplinePoints _splinecomponent))
  (bind _returnvalue_2 (- _returnvalue 1))
  ;[0.15 0.15 0.15 0.5] Init 2 volume pos for end of path
  (Transformation|SetRelativeTransform (Variables|Default|GetStartVolume) (Math|Transform|MakeTransform (Spline|GetLocationatSplinePoint _splinecomponent_2 0 "Local") (Math|Rotator|MakeRotfromX (Class|SplineComponent|GetDirectionatSplinePoint _splinecomponent_2 0 "Local")) "1.000000,1.000000,1.000000") false false)
  (Transformation|SetRelativeTransform (Variables|Default|GetEndVolume) (Math|Transform|MakeTransform (Spline|GetLocationatSplinePoint _splinecomponent _returnvalue_2 "Local") (Math|Rotator|MakeRotfromX (Class|SplineComponent|GetDirectionatSplinePoint _splinecomponent _returnvalue_2 "Local")) "1.000000,1.000000,1.000000") false false))

(fn LeaveSpline
  (params (Actor :type Actor%20Object%20Reference))
  (if (CallFunction|IsActoronSpline Actor)
    (Utilities|Array|RemoveItem (Variables|Default|GetActors) Actor)
    (Default|CallOnActorLeaveSpline Actor)))

(fn JoinSpline
  (params (Actor :type Actor%20Object%20Reference))
  (if (not (CallFunction|IsActoronSpline Actor))
    (Utilities|Array|AddUnique (Variables|Default|GetActors) Actor)
    (Default|CallOnActorJoinSpline Actor)))

(fn IsActoronSpline
  (params (Actor :type Actor%20Object%20Reference%20%28by%20ref%29))
  (return (Utilities|Array|ContainsItem (Variables|Default|GetActors) Actor)))