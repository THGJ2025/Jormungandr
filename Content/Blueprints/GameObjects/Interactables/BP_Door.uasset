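; BP_Door is an interactable door that swings open and closed on alternating interact presses.
; On BeginPlay it registers DoorMesh with its InteractableComponent as an outline mesh.
; Each press runs a FlipFlop that plays or reverses the OpenDoor timeline, whose value scales OpenAngle to set the mesh's relative yaw.
; GetWidgetAttachmentComponent exposes WidgetAttachment as the widget attachment point.
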(event EventInteractPressTriggered
  (Utilities|FlowControl|FlipFlop
    (:A
      (bind _opendoorvalue (Timeline|OpenDoor Play)
        (:Update
          (Transformation|SetRelativeRotation (Variables|Default|GetDoorMesh) (Math|Rotator|MakeRotator 0.0 0.0 (* _opendoorvalue (Variables|Default|GetOpenAngle))) false false))))
    (:B
      (Timeline|OpenDoor Reverse))))

(event EventBeginPlay
  (Class|JInteractableComponent|AddOutlineMeshComponent (Variables|Default|GetInteractableComponent) (Variables|Default|GetDoorMesh)))

(fn ConstructionScript)

(fn GetWidgetAttachmentComponent
  (return (Variables|Default|GetWidgetAttachment)))