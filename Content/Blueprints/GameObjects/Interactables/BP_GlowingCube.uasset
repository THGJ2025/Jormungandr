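; BP_GlowingCube is an interactable cube whose glow toggles when the player interacts with it.
; On BeginPlay it creates a dynamic material instance for the cube mesh and registers that mesh with the InteractableComponent for outlining.
; Press and hold interactions both call their parent events, then share one FlipFlop that switches the material's Emissive parameter on and off.
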(event EventInteractHoldTriggered
  (|CallParentFunction)
  (Utilities|FlowControl|FlipFlop
    (:A
      (Rendering|Material|SetScalarParameterValue (Variables|Default|GetCubeDynamicMaterialInstance) "Emissive" 1.0 :!class /Script/Engine.MaterialInstanceDynamic))
    (:B
      (Rendering|Material|SetScalarParameterValue (Variables|Default|GetCubeDynamicMaterialInstance) "Emissive" 0.0 :!class /Script/Engine.MaterialInstanceDynamic))))

(event EventInteractPressTriggered
  (|CallParentFunction)
  (Utilities|FlowControl|FlipFlop
    (:A
      (Rendering|Material|SetScalarParameterValue (Variables|Default|GetCubeDynamicMaterialInstance) "Emissive" 1.0 :!class /Script/Engine.MaterialInstanceDynamic))
    (:B
      (Rendering|Material|SetScalarParameterValue (Variables|Default|GetCubeDynamicMaterialInstance) "Emissive" 0.0 :!class /Script/Engine.MaterialInstanceDynamic))))

(event EventBeginPlay
  (bind _returnvalue (Rendering|Material|CreateDynamicMaterialInstance (Variables|Default|GetCubeMesh) 0 0 "None" :!class /Script/Engine.PrimitiveComponent))
  (Variables|Default|SetCubeDynamicMaterialInstance _returnvalue)
  (Class|JInteractableComponent|AddOutlineMeshComponent (Variables|Default|GetInteractableComponent) (Variables|Default|GetCubeMesh)))

(fn ConstructionScript)