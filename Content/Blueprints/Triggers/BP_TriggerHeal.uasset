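; BP_TriggerHeal is a trigger that periodically heals actors standing inside its collision component.
; On overlap begin, valid actors with an AC_ActorHealth component join a unique list and start a single looping timer if none exists.
; Each tick of that timer calls Heal on every listed actor by the configured amount and interval.
; Leaving actors are removed, and the timer is cleared once the list is empty.
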(event OnComponentBeginOverlap(CollisionComponent)
  (params (OverlappedComponent :type Primitive%20Component%20Object%20Reference) (OtherActor :type Actor%20Object%20Reference) (OtherComp :type Primitive%20Component%20Object%20Reference) (OtherBodyIndex :type Integer) (bFromSweep :type Boolean) (SweepResult :type Hit%20Result%20Structure%20%28by%20ref%29))
  ;[0.15 0.15 0.15 0.5] Start heal actor on enter trigger
  (Utilities|IsValid OtherActor
    (:Is%20Valid
      (Utilities|IsValid (Actor|GetComponentbyClass OtherActor "/Game/Blueprints/Components/AC_ActorHealth.AC_ActorHealth_C")
        (:Is%20Valid
          (Utilities|Array|AddUnique (Variables|Default|GetActorsToHeal) OtherActor)
          (if (not (Class|KismetSystemLibrary|TimerExistsHandle (Variables|Default|GetHealTimer)))
            (bind _returnvalue (Utilities|Time|SetTimerbyEvent (delegate Custom|HealActors) (Variables|Default|GetHealInterval) true))
            (Variables|Default|SetHealTimer _returnvalue)))))))

(event OnComponentEndOverlap(CollisionComponent)
  (params (OverlappedComponent :type Primitive%20Component%20Object%20Reference) (OtherActor :type Actor%20Object%20Reference) (OtherComp :type Primitive%20Component%20Object%20Reference) (OtherBodyIndex :type Integer))
  (bind _actorstoheal (Variables|Default|GetActorsToHeal))
  ;[0.15 0.15 0.15 0.5] Remove actor to heal once exit trigger
  (Utilities|Array|RemoveItem _actorstoheal OtherActor)
  (if (Utilities|Array|IsEmpty _actorstoheal)
    (Utilities|Time|ClearandInvalidateTimerbyHandle (Variables|Default|GetHealTimer))))

(event Custom|HealActors
  ;[0.15 0.15 0.15 0.5] Heal actors loop
  (for _array_element (Variables|Default|GetActorsToHeal)
    (Default|Heal (Actor|GetComponentbyClass _array_element "/Game/Blueprints/Components/AC_ActorHealth.AC_ActorHealth_C") (Variables|Default|GetHealAmount))))

(fn ConstructionScript)