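; BP_TriggerDamage is a trigger volume that repeatedly damages any actors inside its collision component.
; Begin overlap adds valid actors to a unique list and starts a looping timer at DamageInterval if none is running.
; Each tick of that timer applies Damage to every listed actor, with the trigger as damage causer.
; End overlap removes the actor and clears the timer once the list is empty.
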(event OnComponentBeginOverlap(CollisionComponent)
  (params (OverlappedComponent :type Primitive%20Component%20Object%20Reference) (OtherActor :type Actor%20Object%20Reference) (OtherComp :type Primitive%20Component%20Object%20Reference) (OtherBodyIndex :type Integer) (bFromSweep :type Boolean) (SweepResult :type Hit%20Result%20Structure%20%28by%20ref%29))
  ;[0.15 0.15 0.15 0.5] Start damage actor on enter trigger
  (Utilities|IsValid OtherActor
    (:Is%20Valid
      (Utilities|Array|AddUnique (Variables|Default|GetActorsToDamage) OtherActor)
      (if (not (Class|KismetSystemLibrary|TimerExistsHandle (Variables|Default|GetDamageTimer)))
        (bind _returnvalue (Utilities|Time|SetTimerbyEvent (delegate Custom|DamageActors) (Variables|Default|GetDamageInterval) true))
        (Variables|Default|SetDamageTimer _returnvalue)))))

(event OnComponentEndOverlap(CollisionComponent)
  (params (OverlappedComponent :type Primitive%20Component%20Object%20Reference) (OtherActor :type Actor%20Object%20Reference) (OtherComp :type Primitive%20Component%20Object%20Reference) (OtherBodyIndex :type Integer))
  (bind _actorstodamage (Variables|Default|GetActorsToDamage))
  ;[0.15 0.15 0.15 0.5] Stop damage actor once exit trigger
  (Utilities|Array|RemoveItem _actorstodamage OtherActor)
  (if (Utilities|Array|IsEmpty _actorstodamage)
    (Utilities|Time|ClearandInvalidateTimerbyHandle (Variables|Default|GetDamageTimer))))

(event Custom|DamageActors
  ;[0.15 0.15 0.15 0.5] Damage actors loop
  (for _array_element (Variables|Default|GetActorsToDamage)
    (Game|Damage|ApplyDamage _array_element (Variables|Default|GetDamage) 0 self)))

(fn ConstructionScript)